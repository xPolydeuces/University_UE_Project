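; Paper2D spike trap that endlessly lowers and raises on a timer, damaging actors that touch it while it is up.
; BeginPlay runs a Delay-based loop alternating SpikesDown and SpikesUp, with a Duration variable setting the hold time.
; Each event steps through four sprite frames, then disables or enables the Box collision.
; The Box's begin overlap applies damage to the other actor.
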(event OnComponentBeginOverlap(Box)
  (params (OverlappedComponent :type Primitive%20Component%20Object%20Reference) (OtherActor :type Actor%20Object%20Reference) (OtherComp :type Primitive%20Component%20Object%20Reference) (OtherBodyIndex :type Integer) (bFromSweep :type Boolean) (SweepResult :type Hit%20Result%20Structure%20%28by%20ref%29))
  (Game|Damage|ApplyDamage OtherActor 1.0 0 0))

(event Custom|SpikesDown
  (Rendering|Components|Sprite|SetSprite (Variables|Default|GetPaperSprite) "/Game/Assets/Spikes/Spr_Spikes.Spr_Spikes")
  (Utilities|FlowControl|Delay 0.1)
  (Rendering|Components|Sprite|SetSprite (Variables|Default|GetPaperSprite) "/Game/Assets/Spikes/Spr_Spikes_002.Spr_Spikes_002")
  (Utilities|FlowControl|Delay 0.1)
  (Rendering|Components|Sprite|SetSprite (Variables|Default|GetPaperSprite) "/Game/Assets/Spikes/Spr_Spikes_003.Spr_Spikes_003")
  (Utilities|FlowControl|Delay 0.1)
  (Rendering|Components|Sprite|SetSprite (Variables|Default|GetPaperSprite) "/Game/Assets/Spikes/Spr_Spikes_004.Spr_Spikes_004")
  (Collision|SetCollisionEnabled (Variables|Default|GetBox) "NoCollision"))

(event Custom|SpikesUp
  (Rendering|Components|Sprite|SetSprite (Variables|Default|GetPaperSprite) "/Game/Assets/Spikes/Spr_Spikes_004.Spr_Spikes_004")
  (Utilities|FlowControl|Delay 0.1)
  (Rendering|Components|Sprite|SetSprite (Variables|Default|GetPaperSprite) "/Game/Assets/Spikes/Spr_Spikes_003.Spr_Spikes_003")
  (Utilities|FlowControl|Delay 0.1)
  (Rendering|Components|Sprite|SetSprite (Variables|Default|GetPaperSprite) "/Game/Assets/Spikes/Spr_Spikes_002.Spr_Spikes_002")
  (Utilities|FlowControl|Delay 0.1)
  (Rendering|Components|Sprite|SetSprite (Variables|Default|GetPaperSprite) "/Game/Assets/Spikes/Spr_Spikes.Spr_Spikes")
  (Collision|SetCollisionEnabled (Variables|Default|GetBox) "QueryAndPhysics"))

(event EventBeginPlay
  (|CallParentFunction)
  (CallFunction|SpikesDown :!label _label)
  (Utilities|FlowControl|Delay 0.4)
  (Utilities|FlowControl|Delay (Variables|Default|GetDuration))
  (CallFunction|SpikesUp)
  (Utilities|FlowControl|Delay 0.4)
  (Utilities|FlowControl|Delay (Variables|Default|GetDuration))
  (goto _label))

(event Collision|EventActorBeginOverlap
  (params (OtherActor :type Actor%20Object%20Reference))
  (|CallParentFunction OtherActor) ; This node is disabled and will not be called.\nDrag off pins to build functionality.
)

(event EventTick
  (params (DeltaSeconds :type Float%20%28single-precision%29))
  (|CallParentFunction DeltaSeconds) ; This node is disabled and will not be called.\nDrag off pins to build functionality.
)

(fn ConstructionScript
  (|CallParentFunction))